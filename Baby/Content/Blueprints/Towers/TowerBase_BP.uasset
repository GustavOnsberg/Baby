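; Base tower for a tower defense game that automatically fires projectiles at EnemyBase_BP enemies within its range.
; Overlap events maintain the in-range list, and Tick calls Target on a FireRate delay while the tower is not in hand.
; Target compares track position or health according to TargetMode, pitches TowerParent in the X-Z plane, then calls Fire.
; Range sizes the collision sphere and the range field, which Select and Deselect show or hide.
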(event EventBeginPlay
  (bind _range (Variables|Default|GetRange))
  (bind _returnvalue (/ _range 8192.0))
  (Utilities|FlowControl|Sequence
    (:then_0
      (Transformation|SetRelativeScale3D (Variables|Default|GetRangeField) (Math|Vector|MakeVector _returnvalue _returnvalue _returnvalue))
      (Components|Sphere|SetSphereRadius (Variables|Default|GetRangeCollision) (/ _range 4.0) true))))

(event EventActorBeginOverlap
  (params (OtherActor :type Actor%20Object%20Reference))
  (bind _asenemy_base_bp (Utilities|Casting|CastToEnemyBase_BP OtherActor))
  (Utilities|Array|Add (Variables|Default|GetEnemysInRange) _asenemy_base_bp))

(event EventTick
  (params (DeltaSeconds :type Float%20%28single-precision%29))
  (if (and (Variables|Default|GetCanFire) (not (Variables|Default|GetInHand)))
    (if (> (Utilities|Array|Length (Variables|Default|GetEnemysInRange)) 0)
      (CallFunction|Target)
      (Variables|Default|SetCanFire false)
      (Utilities|FlowControl|Delay (Variables|Default|GetFireRate))
      (Variables|Default|SetCanFire true))))

(event Collision|EventActorEndOverlap
  (params (OtherActor :type Actor%20Object%20Reference))
  (bind _asenemy_base_bp (Utilities|Casting|CastToEnemyBase_BP OtherActor))
  (Utilities|Array|RemoveItem (Variables|Default|GetEnemysInRange) _asenemy_base_bp))

(fn ConstructionScript)

(fn Select
  (if (not (Variables|Default|GetInHand))
    (Variables|Default|SetSelected true)
    (Rendering|SetVisibility (Variables|Default|GetRangeField) true false)))

(fn Deselect
  (if (not (Variables|Default|GetInHand))
    (Variables|Default|SetSelected false)
    (Rendering|SetVisibility (Variables|Default|GetRangeField) false false)))

(fn Target
  (bind _self self)
  (bind _enemysinrange (Variables|Default|GetEnemysInRange))
  (bind _enemysinrange_2 (Variables|Default|GetEnemysInRange))
  (bind _enemysinrange_3 (Variables|Default|GetEnemysInRange))
  (bind _enemysinrange_4 (Variables|Default|GetEnemysInRange))
  (bind _returnvalue (Transformation|GetActorLocation _self))
  (bind (_x _y _z) (Math|Vector|BreakVector _returnvalue))
  (switch int (Variables|Default|GetTargetMode)
    (:0
      ;[1 1 1] Target first
      (for _index (range 0 (Utilities|Array|Length _enemysinrange))
        (if (> (Variables|/Game/Blueprints/Enemys/EnemyBase_BP.EnemyBase_BP_C|GetTrackPosition (Utilities|Array|Get(acopy) _enemysinrange _index)) (Variables|Default|GetTargetComparison))
          (Variables|Default|SetTargetComparison (Variables|/Game/Blueprints/Enemys/EnemyBase_BP.EnemyBase_BP_C|GetTrackPosition (Utilities|Array|Get(acopy) _enemysinrange _index)))
          (Variables|Default|SetTargetEnemy _index))))
    (:1
      ;[1 1 1] Target strong
      (for _index_2 (range 0 (Utilities|Array|Length _enemysinrange_2))
        (if (> (Variables|/Game/Blueprints/Enemys/EnemyBase_BP.EnemyBase_BP_C|GetHealth (Utilities|Array|Get(acopy) _enemysinrange_2 _index_2)) (Variables|Default|GetTargetComparison))
          (Variables|Default|SetTargetComparison (Variables|/Game/Blueprints/Enemys/EnemyBase_BP.EnemyBase_BP_C|GetHealth (Utilities|Array|Get(acopy) _enemysinrange_2 _index_2)))
          (Variables|Default|SetTargetEnemy _index_2))))
    (:2
      ;[1 1 1] Target weak
      (for _index_3 (range 0 (Utilities|Array|Length _enemysinrange_4))
        (if (< (Variables|/Game/Blueprints/Enemys/EnemyBase_BP.EnemyBase_BP_C|GetHealth (Utilities|Array|Get(acopy) _enemysinrange_4 _index_3)) (Variables|Default|GetTargetComparison))
          (Variables|Default|SetTargetComparison (Variables|/Game/Blueprints/Enemys/EnemyBase_BP.EnemyBase_BP_C|GetHealth (Utilities|Array|Get(acopy) _enemysinrange_4 _index_3)))
          (Variables|Default|SetTargetEnemy _index_3))))
    (:3
      (Variables|Default|SetTargetComparison 1e+06)
      ;[1 1 1] Target first
      (for _index_4 (range 0 (Utilities|Array|Length _enemysinrange_3))
        (if (< (Variables|/Game/Blueprints/Enemys/EnemyBase_BP.EnemyBase_BP_C|GetTrackPosition (Utilities|Array|Get(acopy) _enemysinrange_3 _index_4)) (Variables|Default|GetTargetComparison))
          (if (> (Variables|/Game/Blueprints/Enemys/EnemyBase_BP.EnemyBase_BP_C|GetTrackPosition (Utilities|Array|Get(acopy) _enemysinrange_3 _index_4)) 0.0)
            (Variables|Default|SetTargetComparison (Variables|/Game/Blueprints/Enemys/EnemyBase_BP.EnemyBase_BP_C|GetTrackPosition (Utilities|Array|Get(acopy) _enemysinrange_3 _index_4)))
            (Variables|Default|SetTargetEnemy _index_4))))))
  ;[1 1 1] Look at target
  (Variables|Default|SetTargetComparison 0.0)
  (Transformation|SetWorldRotation (Variables|Default|GetTowerParent) (Math|Rotator|MakeRotator 0.0 (+ (Class|KismetMathLibrary|DegAtan2 (- (.Z (Math|Vector|BreakVector (Transformation|GetActorLocation (Utilities|Array|Get(acopy) (Variables|Default|GetEnemysInRange) (Variables|Default|GetTargetEnemy))))) _z) (- (.X (Math|Vector|BreakVector (Transformation|GetActorLocation (Utilities|Array|Get(acopy) (Variables|Default|GetEnemysInRange) (Variables|Default|GetTargetEnemy))))) _x)) -9e+01) 0.0) false false)
  (CallFunction|Fire))

(fn Fire
  (bind _projectilespawnpoint (Variables|Default|GetProjectileSpawnPoint))
  (Game|SpawnActorfromClass (Variables|Default|GetProjectile) (Math|Transform|MakeTransform (Transformation|GetWorldLocation _projectilespawnpoint) (Transformation|GetWorldRotation _projectilespawnpoint) "1,1,1") "AlwaysSpawn" 0 0))

(fn Place
  (bind _returnvalue (Transformation|GetActorLocation))
  (Transformation|SetActorLocation (Math|Vector|MakeVector (.x _returnvalue) 0.0 (.z _returnvalue)) false false))