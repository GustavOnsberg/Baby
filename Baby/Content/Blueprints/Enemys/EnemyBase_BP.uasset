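; Base enemy actor that follows the game mode's track spline and rewards the player when killed.
; BeginPlay caches the Track from GameModeBase_BP and enables movement after a short delay plus StandByTime.
; Tick advances a distance by speed and multiplier, snapping the root to the spline's location and rotation.
; Damage reduces Health; at zero or below it grants Money and XP to Player_BP, recalculates level and destroys itself.
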(event EventBeginPlay
  (Utilities|FlowControl|Sequence
    (:then_0
      (bind _asgame_mode_base_bp (Utilities|Casting|CastToGameModeBase_BP (Game|GetGameMode)))
      (Variables|Default|SetTrack (Variables|/Game/Blueprints/GameModes/GameModeBase_BP.GameModeBase_BP_C|GetTrack _asgame_mode_base_bp)))
    (:then_1
      (Utilities|FlowControl|Delay 0.2)
      (Utilities|FlowControl|Delay (Variables|Default|GetStandByTime))
      (Variables|Default|SetCanMove true))))

(event EventActorBeginOverlap
  (params (OtherActor :type Actor%20Object%20Reference)))

(event EventTick
  (params (DeltaSeconds :type Float%20%28single-precision%29))
  (bind _track (Variables|Default|GetTrack))
  (bind _spline (Variables|/Game/Blueprints/Track_BP.Track_BP_C|GetSpline _track))
  (if (Variables|Default|GetCanMove)
    (bind _output_get (Variables|Default|SetTrackPosition (+ (* DeltaSeconds (Variables|Default|GetSpeed) (Variables|Default|GetSpeedMultiplier)) (Variables|Default|GetTrackPosition))))
    (Transformation|SetWorldLocationAndRotation (Variables|Default|GetDefaultSceneRoot) (Spline|GetLocationatDistanceAlongSpline _spline _output_get "World") (Spline|GetRotationatDistanceAlongSpline _spline _output_get "World") false false)))

(fn ConstructionScript)

(fn Damage
  (params (Damage :type Float%20%28single-precision%29))
  (Variables|Default|SetHealth (- (Variables|Default|GetHealth) Damage))
  (CallFunction|CheckifDead))

(fn CheckifDead
  (if (<= (Variables|Default|GetHealth) 0.0)
    (bind _asplayer_bp (Utilities|Casting|CastToPlayer_BP (Game|Player|GetPlayerPawn 0)))
    (Variables|/Game/Blueprints/Player_BP.Player_BP_C|SetMoney _asplayer_bp (+ (Variables|/Game/Blueprints/Player_BP.Player_BP_C|GetMoney _asplayer_bp) (Variables|Default|GetMoney)))
    (Variables|/Game/Blueprints/Player_BP.Player_BP_C|SetXP _asplayer_bp (+ (Variables|/Game/Blueprints/Player_BP.Player_BP_C|GetXP _asplayer_bp) (Variables|Default|GetXP)))
    (Default|CalculateLevel _asplayer_bp)
    (Actor|DestroyActor)))