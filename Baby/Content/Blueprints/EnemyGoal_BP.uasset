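; EnemyGoal_BP is the goal actor that enemies reach to cost the player lives.
; On BeginPlay it caches the first player pawn as a Player_BP reference.
; When an EnemyBase_BP actor overlaps it, it subtracts that enemy's PlayerDamage from the player's Lifes and destroys the enemy.
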(event EventBeginPlay
  (bind _asplayer_bp (Utilities|Casting|CastToPlayer_BP (Game|Player|GetPlayerPawn 0)))
  (Variables|Default|SetPlayer _asplayer_bp))

(event EventActorBeginOverlap
  (params (OtherActor :type Actor%20Object%20Reference))
  (bind _player (Variables|Default|GetPlayer))
  (bind _asenemy_base_bp (Utilities|Casting|CastToEnemyBase_BP OtherActor))
  (Variables|/Game/Blueprints/Player_BP.Player_BP_C|SetLifes _player (- (Variables|/Game/Blueprints/Player_BP.Player_BP_C|GetLifes _player) (Variables|/Game/Blueprints/Enemys/EnemyBase_BP.EnemyBase_BP_C|GetPlayerDamage _asenemy_base_bp)))
  (Actor|DestroyActor _asenemy_base_bp))

(event EventTick
  (params (DeltaSeconds :type Float%20%28single-precision%29)))

(fn ConstructionScript)