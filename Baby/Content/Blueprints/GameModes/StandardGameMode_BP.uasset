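; Standard game mode that starts a round of enemy spawning as soon as play begins.
; StartNewRound switches on the Round number and calls SpawnEnemy with enemy type, amount and delay; only round one is defined, spawning a single Baby enemy.
; An unconnected chain of larger Baby waves, each waiting on a delay returned by the previous spawn call, never runs.
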(event EventBeginPlay
  (CallFunction|StartNewRound))

(event EventTick
  (params (DeltaSeconds :type Float%20%28single-precision%29)))

(event EventStartNewRound
  (switch int (Variables|Default|GetRound)
    (:1
      (CallFunction|SpawnEnemy "/Game/Blueprints/Enemys/Baby_BP.Baby_BP_C" 1 1.0))))

(fn ConstructionScript
  (|CallParentFunction))