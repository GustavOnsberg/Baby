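; Base projectile actor that flies forward and damages enemies it overlaps.
; Each tick it teleports its root along the actor's forward vector by Speed scaled by delta time, keeping its rotation.
; On overlap with an EnemyBase_BP it calls that enemy's Damage with its Damage value, then destroys itself; other actors are ignored.
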(event EventBeginPlay)

(event EventActorBeginOverlap
  (params (OtherActor :type Actor%20Object%20Reference))
  (bind _asenemy_base_bp (Utilities|Casting|CastToEnemyBase_BP OtherActor))
  (Default|Damage _asenemy_base_bp (Variables|Default|GetDamage))
  (Actor|DestroyActor))

(event EventTick
  (params (DeltaSeconds :type Float%20%28single-precision%29))
  (bind _defaultsceneroot (Variables|Default|GetDefaultSceneRoot))
  (Transformation|SetWorldLocationAndRotation _defaultsceneroot (+ (* (Transformation|GetActorForwardVector) (* DeltaSeconds (Variables|Default|GetSpeed))) (Transformation|GetWorldLocation _defaultsceneroot)) (Transformation|GetWorldRotation _defaultsceneroot) false true))

(fn ConstructionScript)