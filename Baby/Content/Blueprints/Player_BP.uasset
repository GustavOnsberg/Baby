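; Player blueprint that lets the user select towers with the mouse.
; It shows the mouse cursor on BeginPlay, and each left click runs a complex trace under the cursor on the Camera channel.
; A hit TowerBase_BP replaces SelectedTower after the previous one is deselected.
; Any other click deselects the stored tower without clearing the reference, and neither path checks that it is valid.
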(event EventBeginPlay
  (Variables|/Script/Engine.PlayerController|SetbShowMouseCursor (Game|GetPlayerController 0) true))

(event EventActorBeginOverlap
  (params (OtherActor :type Actor%20Object%20Reference)))

(event EventTick
  (params (DeltaSeconds :type Float%20%28single-precision%29)))

(event Input|MouseEvents|LeftMouseButton
  (params (Key :type Key%20Structure :default "AnyKey"))
  (:Pressed
    (bind _astower_base_bp (Utilities|Casting|CastToTowerBase_BP (.hitactor (.HitResult (Game|Player|GetHitResultUnderCursorbyChannel (Game|GetPlayerController 0) "TraceTypeQuery2" true))))
      (:then
        (Default|Deselect (Variables|Default|GetSelectedTower))
        (Default|Select _astower_base_bp)
        (Variables|Default|SetSelectedTower _astower_base_bp))
      (:CastFailed
        (Default|Deselect (Variables|Default|GetSelectedTower))))))

(fn ConstructionScript)